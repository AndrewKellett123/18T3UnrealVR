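; Game state Blueprint that tracks scores for a two-player networked match and shows them on the level's BP_ScoreBoard actor.
; After a two-second delay on BeginPlay, the server writes the first two PlayerArray IDs to the board.
; Score matches the given ID to a player and increments that player's score, with authority only.
; Per-player multicast events copy IDs and scores to every machine's board.
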(event Custom|Score
  (params (ID :type Integer))
  ;[1 0 0] 1 - Set Authority to work from server
  (Networking|SwitchHasAuthority
    (:Authority
      (if (== ID (Variables|/Script/Engine.PlayerState|GetPlayerId (Utilities|Array|Get(acopy) (Variables|Default|GetPlayerArray))))
        (bind _result (Math|Integer|IncrementInt (Variables|Default|GetPlayer%20A%20Score))
          (:%20%20
            (bind _output_get (Variables|/Game/Blueprints/UI/ScoreBoard.ScoreBoard_C|SetScore01 (Variables|/Game/Blueprints/UI/BP_ScoreBoard.BP_ScoreBoard_C|GetBoard (Variables|Default|GetScore%20Board)) _result))
            (CallFunction|UpdateAMulti _output_get)))
        (elif (== ID (Variables|/Script/Engine.PlayerState|GetPlayerId (Utilities|Array|Get(acopy) (Variables|Default|GetPlayerArray) 1)))
          (bind _result_2 (Math|Integer|IncrementInt (Variables|Default|GetPlayer%20B%20Score))
            (:%20%20
              (bind _output_get_2 (Variables|/Game/Blueprints/UI/ScoreBoard.ScoreBoard_C|SetScore02 (Variables|/Game/Blueprints/UI/BP_ScoreBoard.BP_ScoreBoard_C|GetBoard (Variables|Default|GetScore%20Board)) _result_2))
              (CallFunction|UpdateBMulti _output_get_2))))))))

(event Custom|Setup%20B%20Multi
  (params (NewParam :type Integer))
  ;[1 0 0] 2- Multicast result to others
  (Variables|/Game/Blueprints/UI/ScoreBoard.ScoreBoard_C|SetID_02 (Variables|/Game/Blueprints/UI/BP_ScoreBoard.BP_ScoreBoard_C|GetBoard (Variables|Default|GetScore%20Board)) NewParam))

(event Custom|Update%20A%20Multi
  (params (NewParam :type Integer))
  ;[1 0 0] 2- Multicast result to others
  (Variables|/Game/Blueprints/UI/ScoreBoard.ScoreBoard_C|SetScore01 (Variables|/Game/Blueprints/UI/BP_ScoreBoard.BP_ScoreBoard_C|GetBoard (Variables|Default|GetScore%20Board)) NewParam))

(event Custom|Setup%20A%20Multi
  (params (NewParam :type Integer))
  ;[1 0 0] 2- Multicast result to others
  (Variables|/Game/Blueprints/UI/ScoreBoard.ScoreBoard_C|SetID_01 (Variables|/Game/Blueprints/UI/BP_ScoreBoard.BP_ScoreBoard_C|GetBoard (Variables|Default|GetScore%20Board)) NewParam))

(event Custom|Update%20B%20Multi
  (params (NewParam :type Integer))
  ;[1 0 0] 2- Multicast result to others
  (Variables|/Game/Blueprints/UI/ScoreBoard.ScoreBoard_C|SetScore02 (Variables|/Game/Blueprints/UI/BP_ScoreBoard.BP_ScoreBoard_C|GetBoard (Variables|Default|GetScore%20Board)) NewParam))

(event EventBeginPlay
  (bind _outactors (Actor|GetAllActorsOfClass "/Game/Blueprints/UI/BP_ScoreBoard.BP_ScoreBoard_C"))
  (Variables|Default|SetScore%20Board (Utilities|Array|Get(acopy) _outactors))
  (Utilities|FlowControl|Delay 2.0)
  ;[1 0 0] 1 - Set Authority to work from server
  (Networking|SwitchHasAuthority
    (:Authority
      (Utilities|FlowControl|Sequence
        (:then_0
          (bind _output_get (Variables|/Game/Blueprints/UI/ScoreBoard.ScoreBoard_C|SetID_01 (Variables|/Game/Blueprints/UI/BP_ScoreBoard.BP_ScoreBoard_C|GetBoard (Variables|Default|GetScore%20Board)) (Variables|/Script/Engine.PlayerState|GetPlayerId (Utilities|Array|Get(acopy) (Variables|Default|GetPlayerArray)))))
          (CallFunction|SetupAMulti _output_get))
        (:then_1
          (bind _output_get_2 (Variables|/Game/Blueprints/UI/ScoreBoard.ScoreBoard_C|SetID_02 (Variables|/Game/Blueprints/UI/BP_ScoreBoard.BP_ScoreBoard_C|GetBoard (Variables|Default|GetScore%20Board)) (Variables|/Script/Engine.PlayerState|GetPlayerId (Utilities|Array|Get(acopy) (Variables|Default|GetPlayerArray) 1))))
          (CallFunction|SetupBMulti _output_get_2))))))

(event EventTick
  (params (DeltaSeconds :type Float%20%28single-precision%29)))

(fn ConstructionScript)